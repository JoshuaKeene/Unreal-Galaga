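; BP_Enemy_2 is an enemy that steps downward and reverses its movement direction when it hits an obstacle.
; Overlapping the player applies damage and kills the enemy, while overlapping a player projectile just kills it.
; A non-projectile hit pauses movement while a timeline lerps it 100 units down, then re-enables movement with the direction flipped.
; Tick defers to the parent class.
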(event EventBeginPlay
  (|CallParentFunction) ; This node is disabled and will not be called.\nDrag off pins to build functionality.
)

(event Collision|EventActorBeginOverlap
  (params (OtherActor :type Actor%20Object%20Reference))
  ;[1 1 1] Destroying enemy when shot and when colliding with player
  (bind _asbp_player (Utilities|Casting|CastToBP_Player OtherActor)
    (:then
      (Game|Damage|ApplyDamage _asbp_player (Variables|Default|GetDamage) 0 0))
    (:CastFailed
      (Utilities|Casting|CastToBP_ProjectilePlayerBase OtherActor)))
  (CallFunction|EnemyKilled))

(event Collision|EventHit
  (params (MyComp :type Primitive%20Component%20Object%20Reference) (Other :type Actor%20Object%20Reference) (OtherComp :type Primitive%20Component%20Object%20Reference) (bSelfMoved :type Boolean) (HitLocation :type Vector :default "0, 0, 0") (HitNormal :type Vector :default "0, 0, 0") (NormalImpulse :type Vector :default "0, 0, 0") (Hit :type Hit%20Result%20Structure%20%28by%20ref%29))
  ;[1 1 1] Enemy 2 Verticle Movement
  (Utilities|Casting|CastToBP_ProjectilePlayerBase Other
    (:CastFailed
      (Variables|Default|SetActor%20Location (Transformation|GetActorLocation))
      (Variables|Default|SetMoveEnabled false)
      (bind _movedownspeed (Timeline|MoveDownAnimation PlayFromStart)
        (:Update
          (Transformation|SetActorLocation (Math|Vector|Lerp(Vector) (Variables|Default|GetActor%20Location) (- (Variables|Default|GetActor%20Location) "0, 0,100.000000") _movedownspeed) false false))
        (:Finished
          (Variables|Default|SetMoveEnabled true)
          (Variables|Default|SetMoveDirection (not (Variables|Default|GetMoveDirection))))))))

(event EventTick
  (params (DeltaSeconds :type Float%20%28single-precision%29))
  (|CallParentFunction DeltaSeconds))

(fn ConstructionScript
  (|CallParentFunction))