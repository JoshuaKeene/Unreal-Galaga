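; Asteroid enemy that gets a random speed and non-uniform sprite scale on spawn and destroys itself at or below world Z zero.
; Player overlap applies damage, while player projectile overlap rolls for a laser or health pickup drop; both then trigger EnemyKilled.
; The EnemyKilled override spawns an explosion with sound, passes its score value to the game mode and shakes the camera, without adding to the kill count.
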(event EventBeginPlay
  (bind _returnvalue (Math|Random|RandomFloatinRange 0.5 1.0))
  (bind _projectilemovement (Variables|Default|GetProjectileMovement))
  ;[1 1 1] Setting the speed and scale of the asteroids
  (bind _asbp_game_mode (Utilities|Casting|CastToBP_GameMode (Game|GetGameMode)))
  (Variables|Default|SetBP_GameMode _asbp_game_mode)
  (bind _output_get (Variables|Default|SetMoveSpeed (Math|Random|RandomFloatinRange (Variables|Default|GetMinSpeed) (Variables|Default|GetMaxSpeed))))
  (bind _output_get_2 (Variables|/Script/Engine.ProjectileMovementComponent|SetMaxSpeed _projectilemovement _output_get))
  (Variables|/Script/Engine.ProjectileMovementComponent|SetInitialSpeed _projectilemovement _output_get_2)
  (bind _output_get_3 (Variables|Default|SetScale (Math|Vector|MakeVector _returnvalue _returnvalue _returnvalue)))
  (Transformation|SetWorldScale3D (Variables|Default|GetEnemySprite) _output_get_3))

(event Collision|EventActorBeginOverlap
  (params (OtherActor :type Actor%20Object%20Reference))
  (bind _returnvalue (Math|Random|RandomIntegerinRange 1 100))
  (bind _returnvalue_2 (Transformation|GetActorTransform))
  ;[1 1 1] Destroying asteroid when shot and when colliding with player and pick up drop chances and instantiation
  (bind _asbp_player (Utilities|Casting|CastToBP_Player OtherActor)
    (:then
      (Game|Damage|ApplyDamage _asbp_player (Variables|Default|GetDamage) 0 0))
    (:CastFailed
      (Utilities|Casting|CastToBP_ProjectilePlayerBase OtherActor)
      (if (<= (Variables|Default|GetPickUpDropChance) _returnvalue)
        (if (<= (Variables|Default|GetDropTypeChance) _returnvalue)
          (Game|SpawnActorfromClass "/Game/Blueprints/BP_PickUps/BP_LaserDrop.BP_LaserDrop_C" _returnvalue_2 "AlwaysSpawn" 0 0)
          (else
            (Game|SpawnActorfromClass "/Game/Blueprints/BP_PickUps/BP_HealthDrop.BP_HealthDrop_C" _returnvalue_2 "AlwaysSpawn" 0 0))))))
  (CallFunction|EnemyKilled))

(event EventEnemyKilled
  (bind _returnvalue (Transformation|GetActorLocation))
  (bind _bp_gamemode (Variables|Default|GetBP_GameMode))
  ;[1 1 1] Overriding Enemy Killed function so that asteroids do not add to kill count
  (Game|SpawnActorfromClass "/Game/Blueprints/BP_Explosion.BP_Explosion_C" (Transformation|GetWorldTransform (Variables|Default|GetEnemySprite)) "AlwaysSpawn" 0 0)
  (Default|SetScore _bp_gamemode (Variables|Default|GetEnemyScoreValue))
  (Default|PlayCamShake _bp_gamemode "/Game/Blueprints/BP_CameraShake/BP_CamShakeSmall.BP_CamShakeSmall_C" _returnvalue)
  (Audio|PlaySoundatLocation "/Game/Assets/Audio/Explosion.Explosion" _returnvalue)
  (Actor|DestroyActor))

(event EventTick
  (params (DeltaSeconds :type Float%20%28single-precision%29))
  ;[1 1 1] Destroying off screen asteroids
  (Variables|Default|SetMin%20Z 0.0)
  (if (<= (.z (Transformation|GetActorLocation)) (Variables|Default|GetMin%20Z))
    (Actor|DestroyActor)))

(fn ConstructionScript
  (|CallParentFunction))