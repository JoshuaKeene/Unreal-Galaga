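; Trigger-box spawner that populates the game with two enemy types and asteroids at random points in its bounds, keeping Y fixed to the actor's plane.
; Looping timers started on BeginPlay drive enemy and asteroid spawns, each with a random delay.
; Below the GameMode's enemy cap, it spawns type 1 enemies, adding a type 2 at every fifth-kill milestone, guarded against repeats by the stored kill count.
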(event Custom|SpawnEnemy
  (bind _bp_gamemode (Variables|Default|GetBP_GameMode))
  (bind _enemieskilled (Variables|/Game/Blueprints/BP_GameMode.BP_GameMode_C|GetEnemiesKilled _bp_gamemode))
  ;[1 1 1] Checks To See If Conditions Are Correct For Enemy Type 2 Spawn And If Not Spaens Enemy Type 1
  (if (< (Variables|/Game/Blueprints/BP_GameMode.BP_GameMode_C|GetEnemyCount _bp_gamemode) (Variables|/Game/Blueprints/BP_GameMode.BP_GameMode_C|GetMaxEnemies _bp_gamemode))
    (if (and (== (Math|Integer|%(Integer) _enemieskilled 5) 0) (!= _enemieskilled (Variables|Default|GetCurrentEnemiesKilled)))
      (CallFunction|SpawnEnemy2))
    (Utilities|FlowControl|Delay (Math|Random|RandomFloatinRange 0.5 2.0))
    (Game|SpawnActorfromClass "/Game/Blueprints/BP_Enemies/BP_Enemy_1.BP_Enemy_1_C" (Math|Transform|MakeTransform (CallFunction|GetRandomLocation) "0, 0, 0" "1,1,1") "Undefined" 0 0)))

(event Custom|SpawnAsteroid
  ;[1 1 1] Spawns Asteroids
  (for _index (range 0 (Math|Random|RandomIntegerinRange 0 0))
    (Utilities|FlowControl|Delay (Math|Random|RandomFloatinRange 0.5 3.0))
    (Game|SpawnActorfromClass "/Game/Blueprints/BP_Enemies/BP_Enemy_Asteroid.BP_Enemy_Asteroid_C" (Math|Transform|MakeTransform (CallFunction|GetRandomLocation) "0, 0, 0" "1,1,1") "Undefined" 0 0)))

(event Custom|SpawnEnemy_2
  ;[1 1 1] Spawns Enemy Type 2
  (Variables|Default|SetCurrentEnemiesKilled (Variables|/Game/Blueprints/BP_GameMode.BP_GameMode_C|GetEnemiesKilled (Variables|Default|GetBP_GameMode)))
  (Game|SpawnActorfromClass "/Game/Blueprints/BP_Enemies/BP_Enemy_2.BP_Enemy_2_C" (Math|Transform|MakeTransform (CallFunction|GetRandomLocation) "0, 0, 0" "1,1,1") "Undefined" 0 0))

(event EventBeginPlay
  ;[1 1 1] Initiates Spawning On Game Start
  (bind _asbp_game_mode (Utilities|Casting|CastToBP_GameMode (Game|GetGameMode)))
  (Variables|Default|SetBP_GameMode _asbp_game_mode)
  (Utilities|FlowControl|Sequence
    (:then_0
      (Utilities|Time|SetTimerbyFunctionName 0 "SpawnEnemy" 1.0 true))
    (:then_1
      (Utilities|Time|SetTimerbyFunctionName 0 "SpawnAsteroid" 1.0 true))))

(fn ConstructionScript)

(fn GetRandomLocation
  (bind _collisioncomponent (Variables|Default|GetCollisionComponent))
  (bind (_origin _boxextent) (Collision|GetComponentBounds _collisioncomponent))
  (bind _returnvalue (Math|Random|RandomPointinBoundingBox _origin _boxextent))
  ;[1 1 1] Gets Random Location Within Trigger Box
  (return (Math|Vector|MakeVector (.x _returnvalue) (.y (Transformation|GetActorLocation)) (.z _returnvalue))))