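; BP_Enemy_1 is an enemy that fires projectiles at random intervals and dies when hit by the player's shots.
; Tick feeds a randomized 2 to 4 second Delay, acting as a repeating timer that spawns BP_ProjectileEnemyBase at the enemy's transform with a shot sound.
; Overlap with a BP_ProjectilePlayerBase actor calls EnemyKilled, which is not defined in this graph.
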(event EventBeginPlay
  (|CallParentFunction) ; This node is disabled and will not be called.\nDrag off pins to build functionality.
)

(event Collision|EventActorBeginOverlap
  (params (OtherActor :type Actor%20Object%20Reference))
  ;[1 1 1] Destroying enemy when hit by player
  (Utilities|Casting|CastToBP_ProjectilePlayerBase OtherActor)
  (CallFunction|EnemyKilled))

(event EventTick
  (params (DeltaSeconds :type Float%20%28single-precision%29))
  ;[1 1 1] Enemy Shooting
  (|CallParentFunction DeltaSeconds)
  (Utilities|FlowControl|Delay (Math|Random|RandomFloatinRange 2.0 4.0))
  (Game|SpawnActorfromClass "/Game/Blueprints/BP_Projectiles/BP_ProjectileEnemyBase.BP_ProjectileEnemyBase_C" (Transformation|GetActorTransform) "Undefined" 0 0)
  (Audio|PlaySoundatLocation "/Game/Assets/Audio/EnemyShot.EnemyShot" (Transformation|GetActorLocation)))

(fn ConstructionScript
  (|CallParentFunction))