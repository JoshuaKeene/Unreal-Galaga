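; Base enemy Blueprint that registers with BP_GameMode's enemy count and dies when overlapped by a player projectile.
; On spawn, a timeline lowers it into position, then enables swept sideways movement along X at a random speed and direction, reversing on hits from anything other than player projectiles.
; Death spawns an explosion with sound and calls the game mode for kill tracking, score and camera shake before destroying the actor.
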(event EventBeginPlay
  ;[1 1 1] Setup References and Variables
  (bind _asbp_game_mode (Utilities|Casting|CastToBP_GameMode (Game|GetGameMode)))
  (bind _output_get (Variables|Default|SetBP_GameMode _asbp_game_mode))
  (Default|UpdateEnemyCount _output_get 1)
  (Variables|Default|SetMoveDirection (Math|Random|RandomBool))
  (Variables|Default|SetMoveSpeed (Math|Random|RandomFloatinRange (Variables|Default|GetMinSpeed) (Variables|Default|GetMaxSpeed)))
  (Variables|Default|SetSpawnLocation (Transformation|GetActorLocation))
  ;[1 1 1] Spawn Animation
  (bind _entryspeed (Timeline|SpawnAnimation Play)
    (:Update
      (Transformation|SetActorLocation (Math|Vector|Lerp(Vector) (Variables|Default|GetSpawnLocation) (- (Variables|Default|GetSpawnLocation) "0, 0,120.000000") _entryspeed) false false))
    (:Finished
      (Variables|Default|SetMoveEnabled true))))

(event Collision|EventActorBeginOverlap
  (params (OtherActor :type Actor%20Object%20Reference))
  ;[1 1 1] Destroying enemy when hit by player
  (Utilities|Casting|CastToBP_ProjectilePlayerBase OtherActor)
  (CallFunction|EnemyKilled))

(event EventTick
  (params (DeltaSeconds :type Float%20%28single-precision%29))
  ;[1 1 1] Basic Sideways Movement
  (CallFunction|EnemyMovement DeltaSeconds))

(event Collision|EventHit
  (params (MyComp :type Primitive%20Component%20Object%20Reference) (Other :type Actor%20Object%20Reference) (OtherComp :type Primitive%20Component%20Object%20Reference) (bSelfMoved :type Boolean) (HitLocation :type Vector :default "0, 0, 0") (HitNormal :type Vector :default "0, 0, 0") (NormalImpulse :type Vector :default "0, 0, 0") (Hit :type Hit%20Result%20Structure%20%28by%20ref%29))
  ;[1 1 1] Basic Sideways Movement
  (Utilities|Casting|CastToBP_ProjectilePlayerBase Other
    (:CastFailed
      (Variables|Default|SetMoveDirection (not (Variables|Default|GetMoveDirection))))))

(fn ConstructionScript)

(fn EnemyKilled
  (bind _returnvalue (Transformation|GetActorLocation))
  (bind _bp_gamemode (Variables|Default|GetBP_GameMode))
  ;[1 1 1] Destroys Enemy, Updates Score, Performs Camera Shake, Plays Audio.
  (Game|SpawnActorfromClass "/Game/Blueprints/BP_Explosion.BP_Explosion_C" (Transformation|GetWorldTransform (Variables|Default|GetEnemySprite)) "AlwaysSpawn" 0 0)
  (Default|EnemyKilled _bp_gamemode)
  (Default|SetScore _bp_gamemode (Variables|Default|GetEnemyScoreValue))
  (Default|PlayCamShake _bp_gamemode "/Game/Blueprints/BP_CameraShake/BP_CamShakeSmall.BP_CamShakeSmall_C" _returnvalue)
  (Audio|PlaySoundatLocation "/Game/Assets/Audio/Explosion.Explosion" _returnvalue)
  (Actor|DestroyActor))

(fn EnemyMovement
  (params (Delta%20Seconds :type Float%20%28single-precision%29))
  (if (Variables|Default|GetMoveEnabled)
    (Transformation|SetActorLocation (+ (Transformation|GetActorLocation) (* (Math|Vector|MakeVector (* (Variables|Default|GetMoveSpeed) (Math|Float|SelectFloat 1.0 -1.0 (Variables|Default|GetMoveDirection))) 0.0 0.0) Delta%20Seconds)) true false)))