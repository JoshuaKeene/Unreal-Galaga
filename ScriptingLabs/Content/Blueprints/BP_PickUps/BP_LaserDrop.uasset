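; Laser power-up pickup actor that activates the player's drop power-up on contact.
; On BeginPlay it caches the game mode, applies MoveSpeed to its projectile movement and scales its sprite by PickUpScale.
; Overlapping BP_Player sets that player's DropActive flag and destroys the pickup.
; Tick also destroys it once its Z position reaches zero or below, treated as off screen.
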(event EventBeginPlay
  (bind _pickupscale (Variables|Default|GetPickUpScale))
  (bind _projectilemovement (Variables|Default|GetProjectileMovement))
  ;[1 1 1] Movement and scale
  (bind _asbp_game_mode (Utilities|Casting|CastToBP_GameMode (Game|GetGameMode)))
  (Variables|Default|SetBP_GameMode _asbp_game_mode)
  (bind _output_get (Variables|Default|SetMoveSpeed (Variables|Default|GetMoveSpeed)))
  (bind _output_get_2 (Variables|/Script/Engine.ProjectileMovementComponent|SetMaxSpeed _projectilemovement _output_get))
  (Variables|/Script/Engine.ProjectileMovementComponent|SetInitialSpeed _projectilemovement _output_get_2)
  (bind _output_get_3 (Variables|Default|SetScale (Math|Vector|MakeVector _pickupscale _pickupscale _pickupscale)))
  (Transformation|SetWorldScale3D (Variables|Default|GetDropSprite) _output_get_3))

(event Collision|EventActorBeginOverlap
  (params (OtherActor :type Actor%20Object%20Reference))
  ;[1 1 1] Applying power up to player
  (bind _asbp_player (Utilities|Casting|CastToBP_Player OtherActor))
  (Variables|/Game/Blueprints/BP_Player.BP_Player_C|SetDropActive _asbp_player true)
  (Actor|DestroyActor))

(event EventTick
  (params (DeltaSeconds :type Float%20%28single-precision%29))
  ;[1 1 1] Destroying Once Off Screen
  (Variables|Default|SetMin%20Z 0.0)
  (if (<= (.z (Transformation|GetActorLocation)) (Variables|Default|GetMin%20Z))
    (Actor|DestroyActor)))

(fn ConstructionScript)