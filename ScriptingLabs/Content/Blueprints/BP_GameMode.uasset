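; Game mode Blueprint that tracks score and enemy counts and manages the game's UI screens and pause state.
; Helper functions create start, controls, HUD, pause and game-over widgets, with menus switching to UI-only input and a visible cursor.
; It also plays world camera shakes at a given epicenter.
; LoadScore and SaveScore are empty stubs, and SetScore adds to Score but overwrites TopScore in both branches.
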(event EventBeginPlay
  (Input|SetInputModeGameOnly (Game|GetPlayerController 0))
  (CallFunction|LoadScore)
  (CallFunction|SetScore))

(event EventTick
  (params (DeltaSeconds :type Float%20%28single-precision%29)))

(event EventEndPlay
  (params (EndPlayReason :type EEndPlayReason%20Enum :default "Destroyed"))
  (CallFunction|SaveScore))

(fn ConstructionScript)

(fn LoadScore)

(fn SaveScore)

(fn SetScore
  (params (Val :type Integer))
  (bind _output_get (Variables|Default|SetScore (+ Val (Variables|Default|GetScore))))
  (if (>= _output_get (Variables|Default|GetTopScore))
    (Variables|Default|SetTopScore (Variables|Default|GetScore))
    (else
      (Variables|Default|SetTopScore (Variables|Default|GetScore)))))

(fn UpdateEnemyCount
  (params (B :type Integer))
  (Variables|Default|SetEnemyCount (+ (Variables|Default|GetEnemyCount) B)))

(fn PlayCamShake
  (params (Shake :type Camera%20Shake%20Class%20Reference) (Epicenter :type Vector))
  (Camera|PlayWorldCameraShake Shake Epicenter 0.0 1e+03))

(fn GameOver
  (bind _returnvalue (Game|GetPlayerController 0))
  (bind _returnvalue_2 (UserInterface|CreateWidget "/Game/Blueprints/BP_UserInterface/BPW_GameOver.BPW_GameOver_C"))
  (UserInterface|Viewport|AddtoViewport _returnvalue_2 0)
  (Variables|/Script/Engine.PlayerController|SetbShowMouseCursor _returnvalue true)
  (Input|SetInputModeUIOnly _returnvalue _returnvalue_2 "DoNotLock"))

(fn EnemyKilled
  (Math|Integer|IncrementInt (Variables|Default|GetEnemiesKilled)
    (:%20%20
      (CallFunction|UpdateEnemyCount -1))))

(fn StartMenu
  (bind _returnvalue (Game|GetPlayerController 0))
  (bind _returnvalue_2 (UserInterface|CreateWidget "/Game/Blueprints/BP_UserInterface/BPW_GameStart.BPW_GameStart_C"))
  (UserInterface|Viewport|AddtoViewport _returnvalue_2 0)
  (Variables|/Script/Engine.PlayerController|SetbShowMouseCursor _returnvalue true)
  (Input|SetInputModeUIOnly _returnvalue _returnvalue_2 "DoNotLock"))

(fn GameHUD
  (bind _returnvalue (UserInterface|CreateWidget "/Game/Blueprints/BP_UserInterface/BPW_HUD.BPW_HUD_C"))
  (bind _output_get (Variables|Default|SetBPW_HUD _returnvalue))
  (UserInterface|Viewport|AddtoViewport _output_get 0))

(fn ControlsMenu
  (bind _returnvalue (Game|GetPlayerController 0))
  (bind _returnvalue_2 (UserInterface|CreateWidget "/Game/Blueprints/BP_UserInterface/BPW_ControlsMenu.BPW_ControlsMenu_C"))
  (UserInterface|Viewport|AddtoViewport _returnvalue_2 0)
  (Variables|/Script/Engine.PlayerController|SetbShowMouseCursor _returnvalue true)
  (Input|SetInputModeUIOnly _returnvalue _returnvalue_2 "DoNotLock"))

(fn GamePaused
  (bind _returnvalue (Game|GetPlayerController 0))
  (bind _returnvalue_2 (UserInterface|CreateWidget "/Game/Blueprints/BP_UserInterface/BPW_GamePaused.BPW_GamePaused_C"))
  (bind _output_get (Variables|Default|SetBPW_GamePaused _returnvalue_2))
  (UserInterface|Viewport|AddtoViewport _output_get 0)
  (Variables|/Script/Engine.PlayerController|SetbShowMouseCursor _returnvalue true)
  (Input|SetInputModeUIOnly _returnvalue _returnvalue_2 "DoNotLock")
  (Game|SetGamePaused true))

(fn GameResume
  (bind _returnvalue (Game|GetPlayerController 0))
  (Widget|RemovefromParent (Variables|Default|GetBPW_GamePaused))
  (Variables|/Script/Engine.PlayerController|SetbShowMouseCursor _returnvalue false)
  (Game|SetGamePaused false)
  (Input|SetInputModeGameOnly _returnvalue))