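; Base Blueprint for player projectiles, which handles their speed and cleanup.
; The Construction Script copies the Speed variable into the max and initial speed of the ProjectileMovement component.
; The projectile destroys itself when Tick finds it at or above a fixed world Z limit, treated as off screen, or when its SP_Rocket component begins any overlap.
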(event OnComponentBeginOverlap(SP_Rocket)
  (params (OverlappedComponent :type Primitive%20Component%20Object%20Reference) (OtherActor :type Actor%20Object%20Reference) (OtherComp :type Primitive%20Component%20Object%20Reference) (OtherBodyIndex :type Integer) (bFromSweep :type Boolean) (SweepResult :type Hit%20Result%20Structure%20%28by%20ref%29))
  ;[1 1 1] Destorying Off Screen Projectiles
  (Actor|DestroyActor))

(event EventTick
  (params (DeltaSeconds :type Float%20%28single-precision%29))
  ;[1 1 1] Destorying Off Screen Projectiles
  (Variables|Default|SetMax%20Z 4.8e+02)
  (if (>= (.z (Transformation|GetActorLocation)) (Variables|Default|GetMax%20Z))
    (Actor|DestroyActor)))

(fn ConstructionScript
  (bind _projectilemovement (Variables|Default|GetProjectileMovement))
  ;[1 1 1] Projectile Movement
  (bind _output_get (Variables|/Script/Engine.ProjectileMovementComponent|SetMaxSpeed _projectilemovement (Variables|Default|GetSpeed)))
  (Variables|/Script/Engine.ProjectileMovementComponent|SetInitialSpeed _projectilemovement _output_get))