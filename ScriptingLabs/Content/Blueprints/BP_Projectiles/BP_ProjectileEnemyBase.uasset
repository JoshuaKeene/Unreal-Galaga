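; BP_ProjectileEnemyBase is an enemy laser projectile, apparently a base class, that damages the player on contact.
; The construction script sets the projectile movement's initial and max speed from its Speed variable.
; An overlap on SP_Laser applies Damage if the other actor is BP_Player, then destroys the projectile whatever it hit.
; Tick also destroys it once its Z position drops to zero or below, treated as off screen.
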(event OnComponentBeginOverlap(SP_Laser)
  (params (OverlappedComponent :type Primitive%20Component%20Object%20Reference) (OtherActor :type Actor%20Object%20Reference) (OtherComp :type Primitive%20Component%20Object%20Reference) (OtherBodyIndex :type Integer) (bFromSweep :type Boolean) (SweepResult :type Hit%20Result%20Structure%20%28by%20ref%29))
  ;[1 1 1] Applying Damage to Player
  (bind _asbp_player (Utilities|Casting|CastToBP_Player OtherActor)
    (:then
      (Game|Damage|ApplyDamage _asbp_player (Variables|Default|GetDamage) 0 0))
    (:CastFailed
      _))
  ;[1 1 1] Destorying Off Screen Projectiles
  (Actor|DestroyActor))

(event EventTick
  (params (DeltaSeconds :type Float%20%28single-precision%29))
  ;[1 1 1] Destorying Off Screen Projectiles
  (Variables|Default|SetMin%20Z 0.0)
  (if (<= (.z (Transformation|GetActorLocation)) (Variables|Default|GetMin%20Z))
    (Actor|DestroyActor)))

(fn ConstructionScript
  (bind _projectilemovement (Variables|Default|GetProjectileMovement))
  ;[1 1 1] Projectile Movement
  (bind _output_get (Variables|/Script/Engine.ProjectileMovementComponent|SetMaxSpeed _projectilemovement (Variables|Default|GetSpeed)))
  (Variables|/Script/Engine.ProjectileMovementComponent|SetInitialSpeed _projectilemovement _output_get))