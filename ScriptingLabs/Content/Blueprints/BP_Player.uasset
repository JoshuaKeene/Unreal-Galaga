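; Player ship Blueprint for a side-to-side shooter, handling movement, shooting, damage and death.
; A timeline raises it on spawn before enabling firing, while Tick applies interpolated horizontal input as swept movement.
; Primary fire is a cooldown-limited single shot, swapped for uncooled twin lasers while the timed DropActive pickup runs; secondary fires a slower triple shot.
; Damage reduces clamped health with camera shake and sound, calling GameOver on the game mode at zero.
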(event Custom|SecFire
  ;[1 1 1] Player Shooting Input - Secondary Fire
  (CallFunction|SecondaryFire (Transformation|GetWorldTransform (Variables|Default|GetProjectileSpawn)))
  (CallFunction|SecondaryFire (Transformation|GetWorldTransform (Variables|Default|GetProjectileSpawnL)))
  (CallFunction|SecondaryFire (Transformation|GetWorldTransform (Variables|Default|GetProjectileSpawnR)))
  (Variables|Default|SetShooting%20Cooldown (+ (Utilities|Time|GetGameTimeinSeconds) 0.5)))

(event Custom|CustomEvent
  ;[1 1 1] Player Shooting Input - Primary Fire
  ;;[1 1 1] PickUpFireMode
  (CallFunction|PrimaryFire (Transformation|GetWorldTransform (Variables|Default|GetProjectileSpawnL)))
  (CallFunction|PrimaryFire (Transformation|GetWorldTransform (Variables|Default|GetProjectileSpawnR))))

(event Custom|PrimFire
  ;[1 1 1] Player Shooting Input - Primary Fire
  (CallFunction|PrimaryFire (Transformation|GetWorldTransform (Variables|Default|GetProjectileSpawn)))
  (Variables|Default|SetShooting%20Cooldown (+ (Utilities|Time|GetGameTimeinSeconds) 0.2)))

(event EventBeginPlay
  ;[1 1 1] Player Spawn Animation
  (bind _asbp_game_mode (Utilities|Casting|CastToBP_GameMode (Game|GetGameMode)))
  (Variables|Default|SetBP_GameMode _asbp_game_mode)
  (Variables|Default|SetSpawnLocation (Transformation|GetActorLocation))
  (bind _speed (Timeline|SpawnAnimation Play)
    (:Update
      (Transformation|SetActorLocation (Math|Vector|Lerp(Vector) (Variables|Default|GetSpawnLocation) (+ (Variables|Default|GetSpawnLocation) "0, 0,60.000000") _speed) false false))
    (:Finished
      (Variables|Default|SetMoveEnabled true))))

(event EventTick
  (params (DeltaSeconds :type Float%20%28single-precision%29))
  ;[1 1 1] Player Movement
  (Utilities|FlowControl|Sequence
    (:then_0
      _)
    (:then_1
      (if (Variables|Default|GetDropActive)
        (Utilities|FlowControl|Delay 1e+01)
        (Variables|Default|SetDropActive false))))
  (Variables|Default|SetDeltaSeconds DeltaSeconds)
  (Transformation|SetActorLocation (+ (Transformation|GetActorLocation) (Math|Vector|MakeVector (Variables|Default|GetHozSpeed) 0.0 0.0)) true false))

(event Game|Damage|EventAnyDamage
  (params (Damage :type Float%20%28single-precision%29) (DamageType :type Damage%20Type%20Object%20Reference) (InstigatedBy :type Controller%20Object%20Reference) (DamageCauser :type Actor%20Object%20Reference))
  ;[1 1 1] Player death and taking damage
  (CallFunction|PlayerDamage Damage))

(event Input|ActionEvents|InputActionPrimaryFire
  (params (Key :type Key%20Structure))
  ;[1 1 1] Player Shooting Input - Primary Fire
  (:Pressed
    (if (Variables|Default|GetMoveEnabled)
      (if (Variables|Default|GetDropActive)
        ;;[1 1 1] PickUpFireMode
        (CallFunction|PrimaryFire (Transformation|GetWorldTransform (Variables|Default|GetProjectileSpawnL)))
        (CallFunction|PrimaryFire (Transformation|GetWorldTransform (Variables|Default|GetProjectileSpawnR)))
        (else
          (Math|Float|CompareFloat (Variables|Default|GetShooting%20Cooldown) (Utilities|Time|GetGameTimeinSeconds)
            (:<
              (CallFunction|PrimaryFire (Transformation|GetWorldTransform (Variables|Default|GetProjectileSpawn)))
              (Variables|Default|SetShooting%20Cooldown (+ (Utilities|Time|GetGameTimeinSeconds) 0.2))))))))
  (:Released
    (Utilities|Time|ClearTimerbyFunctionName 0 "PrimFire")))

(event Input|ActionEvents|InputActionSecondaryFire
  (params (Key :type Key%20Structure))
  ;[1 1 1] Player Shooting Input - Secondary Fire
  (:Pressed
    (if (Variables|Default|GetMoveEnabled)
      (Math|Float|CompareFloat (Variables|Default|GetShooting%20Cooldown) (Utilities|Time|GetGameTimeinSeconds)
        (:<
          (CallFunction|SecondaryFire (Transformation|GetWorldTransform (Variables|Default|GetProjectileSpawn)))
          (CallFunction|SecondaryFire (Transformation|GetWorldTransform (Variables|Default|GetProjectileSpawnL)))
          (CallFunction|SecondaryFire (Transformation|GetWorldTransform (Variables|Default|GetProjectileSpawnR)))
          (Variables|Default|SetShooting%20Cooldown (+ (Utilities|Time|GetGameTimeinSeconds) 0.5))))))
  (:Released
    (Utilities|Time|ClearTimerbyFunctionName 0 "SecFire")))

(event Input|AxisEvents|InputAxisMoveRight
  (params (AxisValue :type Float%20%28single-precision%29))
  (bind _deltaseconds (Variables|Default|GetDeltaSeconds))
  ;[1 1 1] Player Movement Input
  (Variables|Default|SetHozSpeed (Math|Interpolation|FInterpTo (Variables|Default|GetHozSpeed) (* (* (Variables|Default|GetMovementSpeed) AxisValue) _deltaseconds) _deltaseconds 8.0)))

(fn ConstructionScript
  ;[1 1 1] Setting Max Health
  (Variables|Default|SetHealth (Variables|Default|GetMaxHealth)))

(fn PrimaryFire
  (params (SpawnTransform :type Transform))
  ;[1 1 1] Projectile Spawn
  (if (Variables|Default|GetDropActive)
    (Game|SpawnActorfromClass "/Game/Blueprints/BP_Projectiles/BP_ProjectilePlayerBase_LaserChild.BP_ProjectilePlayerBase_LaserChild_C" SpawnTransform "AlwaysSpawn" 0 self)
    (else
      (Game|SpawnActorfromClass "/Game/Blueprints/BP_Projectiles/BP_ProjectilePlayerBase.BP_ProjectilePlayerBase_C" SpawnTransform "AlwaysSpawn" 0 self)))
  (Audio|PlaySoundatLocation "/Game/Assets/Audio/Shot.Shot" (Transformation|GetActorLocation)))

(fn SecondaryFire
  (params (Spawn :type Transform))
  ;[1 1 1] Projectile Spawn
  (Game|SpawnActorfromClass "/Game/Blueprints/BP_Projectiles/BP_ProjectilePlayerBase.BP_ProjectilePlayerBase_C" Spawn "AlwaysSpawn" 0 self)
  (Audio|PlaySoundatLocation "/Game/Assets/Audio/Shot.Shot" (Transformation|GetActorLocation)))

(fn PlayerDamage
  (params (Damage :type Float%20%28single-precision%29))
  (bind _returnvalue (Transformation|GetActorLocation))
  (bind _returnvalue_2 (Transformation|GetActorLocation))
  (bind _bp_gamemode (Variables|Default|GetBP_GameMode))
  (Variables|Default|SetHealth (Math|Float|Clamp(Float) (- (Variables|Default|GetHealth) Damage) 0.0 (Variables|Default|GetMaxHealth)))
  (Default|PlayCamShake (Variables|Default|GetBP_GameMode) "/Game/Blueprints/BP_CameraShake/BP_CamShake.BP_CamShake_C" _returnvalue_2)
  (Audio|PlaySoundatLocation "/Game/Assets/Audio/Explosion.Explosion" _returnvalue_2)
  (if (<= (Variables|Default|GetHealth) 0.0)
    (Game|SpawnActorfromClass "/Game/Blueprints/BP_Explosion.BP_Explosion_C" (Transformation|GetWorldTransform (Variables|Default|GetPlayerSprite)) "AlwaysSpawn" 0 0)
    (Audio|PlaySoundatLocation "/Game/Assets/Audio/Explosion.Explosion" _returnvalue)
    (Default|PlayCamShake _bp_gamemode "/Game/Blueprints/BP_CameraShake/BP_CamShake.BP_CamShake_C" _returnvalue)
    (Default|GameOver _bp_gamemode)
    (Actor|DestroyActor)))